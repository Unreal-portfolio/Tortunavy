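; BP_PGSpiner is a Builder Blueprint that spins its Stick1 component around the yaw axis.
; BeginPlay stores Stick1's starting relative rotation, then calls a custom event that plays a Timeline.
; Each Timeline update sets the relative yaw by lerping from the initial yaw to that yaw plus RotationAngle, using the Rotation track as alpha.
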(event `self.ReceiveBeginPlay`
  (set `self.InitialRotation` (`SceneComponent.RelativeRotation` (`self.Stick1`)))
  (`self.CE_RotateS1`))

(event `CE_RotateS1`
  (bind (_initialrotation_roll _initialrotation_pitch _initialrotation_yaw) (`KismetMathLibrary.BreakRotator` (`self.InitialRotation`)))
  (bind (_direction _rotation) (`Timeline|Timeline`)
    (:`Update`
      (`SceneComponent.K2_SetRelativeRotation` (`self.Stick1`) (`KismetMathLibrary.MakeRotator` 0.0 0.0 (`KismetMathLibrary.Lerp` _initialrotation_yaw (+ _initialrotation_yaw (`self.RotationAngle`)) _rotation)) false false))))

(fn `UserConstructionScript`)